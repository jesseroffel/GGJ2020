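; Shared two-player camera controller that keeps both train players framed by following their midpoint and zooming with their spread.
; Each tick, the Parent component lerps toward the midpoint of TrainPlayer1 and TrainPlayer2, read from GM_Gamemode.
; The camera separately lerps to an offset above Parent, with height range-mapped and clamped from the farther player character's distance to Parent.
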(event `self.ReceiveBeginPlay`
  (bind _asgm_gamemode (cast `/Game/Blueprints/GM_Gamemode` (`GameplayStatics.GetGameMode`)))
  (set `self.Gamemode` _asgm_gamemode))

(event `self.ReceiveTick`
  (params (DeltaSeconds :type "Float (single-precision)"))
  (bind _middlepoint (`self.GetMiddlePoint`))
  (`self.Movement` _middlepoint DeltaSeconds)
  (bind _zoompoint (`self.GetZoomPoint`))
  (`self.Zoom` _zoompoint DeltaSeconds))

(fn `GetMiddlePoint`
  (returns (MiddlePoint :type "Vector Structure"))
  (bind _gamemode (`self.Gamemode`))
  (bind _returnvalue (`self.K2_GetActorLocation` (`/Game/Blueprints/GM_Gamemode.TrainPlayer1` _gamemode)))
  (bind _returnvalue_2 (`self.K2_GetActorLocation` (`/Game/Blueprints/GM_Gamemode.TrainPlayer2` _gamemode)))
  (return (+ (* (`KismetMathLibrary.Normal` (- _returnvalue _returnvalue_2)) (/ (`KismetMathLibrary.Vector_Distance` _returnvalue _returnvalue_2) 2.0)) _returnvalue_2)))

(fn `GetZoomPoint`
  (returns (ZoomPoint :type "Vector Structure"))
  (locals (BigestDistance :type "Float (double-precision)"))
  (bind (_x _y) (`KismetMathLibrary.BreakVector2D` (`self.DistanceMiddlePointMinMax`)))
  (bind (_x_2 _y_2) (`KismetMathLibrary.BreakVector2D` (`self.ZoomMinMax`)))
  (bind _returnvalue (`SceneComponent.K2_GetComponentLocation` (`self.Parent`)))
  (bind _returnvalue_2 (`KismetMathLibrary.Vector_Distance` _returnvalue (`self.K2_GetActorLocation` (`GameplayStatics.GetPlayerCharacter` 1))))
  (bind _returnvalue_3 (`KismetMathLibrary.Vector_Distance` (`self.K2_GetActorLocation` (`GameplayStatics.GetPlayerCharacter` 0)) _returnvalue))
  (if (> _returnvalue_3 _returnvalue_2)
    (set `local.BigestDistance` _returnvalue_3)
    (else
      (set `local.BigestDistance` _returnvalue_2)))
  (if (< (`local.BigestDistance`) (`KismetMathLibrary.BreakVector2D` (`self.DistanceMiddlePointMinMax`)))
    (return (+ (`KismetMathLibrary.MakeVector` 0.0 0.0 (`KismetMathLibrary.BreakVector2D` (`self.ZoomMinMax`))) (+ (`SceneComponent.K2_GetComponentLocation` (`self.Parent`)) (`self.OffsetCamera`))))
    (else
      (return (+ (`KismetMathLibrary.MakeVector` 0.0 0.0 (`KismetMathLibrary.MapRangeClamped` (`local.BigestDistance`) _x _y _x_2 _y_2)) (+ (`SceneComponent.K2_GetComponentLocation` (`self.Parent`)) (`self.OffsetCamera`)))))))

(fn `Movement`
  (params (TargetLocation :type "Vector Structure") (DeltaTime :type "Float (double-precision)"))
  (`SceneComponent.K2_SetWorldLocation` (`self.Parent`) (`KismetMathLibrary.VLerp` (`SceneComponent.K2_GetComponentLocation` (`self.Parent`)) TargetLocation (* DeltaTime (`self.MovementSpeed`))) false false))

(fn `UserConstructionScript`)

(fn `Zoom`
  (params (TargetLocation :type "Vector Structure") (DeltaTime :type "Float (double-precision)"))
  (`SceneComponent.K2_SetWorldLocation` (`self.Camera`) (`KismetMathLibrary.VLerp` (`SceneComponent.K2_GetComponentLocation` (`self.Camera`)) TargetLocation (* DeltaTime (`self.ZoomSpeed`))) false false))