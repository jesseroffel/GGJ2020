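; Component that runs quick time events on interactables: button mashing, button sequences or single presses.
; SetQuickTimeEvent spawns a BP_InteractiveWidget at the interactable and picks random required buttons.
; Tick checks the key from SetButtonPress against two bindings per button, decaying the mash bar or resetting sequences on wrong presses.
; Success destroys the widget actor and notifies the player; ButtonFail only stops the event and logs it.
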(event `self.ReceiveTick`
  (params (DeltaSeconds :type "Float (single-precision)"))
  (bind _lastkeypressed (`self.LastKeyPressed`))
  (bind _lastkeypressed_2 (`self.LastKeyPressed`))
  (bind _buttonsequenceindex (`self.ButtonSequenceIndex`))
  (bind _lastkeypressed_3 (`self.LastKeyPressed`))
  ;[1 1 1] Onupdate
  (if (`self.EventActive`)
    (if (not (`self.FailedEvent`))
      (switch `/Game/Blueprints/Player/E_EventType` (`self.CurrentQuickTimeEvent`)
        (:`NewEnumerator0`
          ;[1 1 1] ButtonMashing
          (if (== _lastkeypressed_2 "None")
            (`self.SubtractTotalButtonPress` (* (`self.ButtonMashDecay`) DeltaSeconds))
            (`/Game/Widgets/W_QuickTimeEvent.SetMashingBar` (`self.QuickTimeEventWidget`) (`self.ButtonPressCount`))
            (else
              (bind _keypressed (`self.CheckForInput` _lastkeypressed_2 "NewEnumerator4"))
              (if _keypressed
                (set `self.ButtonPressCount` (+ (`self.ButtonPressCount`) (`self.ButtonMashSuccess`)))
                (if (>= (`self.ButtonPressCount`) (`self.TotalButtonPressCount`))
                  (`self.FinishEventHandling`)
                  (else
                    (set `self.LastKeyPressed` "None")
                    (`/Game/Widgets/W_QuickTimeEvent.SetMashingBar` (`self.QuickTimeEventWidget`) (`self.ButtonPressCount`))))
                (else
                  (`self.SubtractTotalButtonPress` (`self.ButtonFailDecrement`))
                  (set `self.LastKeyPressed` "None")
                  (`/Game/Widgets/W_QuickTimeEvent.SetMashingBar` (`self.QuickTimeEventWidget`) (`self.ButtonPressCount`)))))))
        (:`NewEnumerator1`
          ;[1 1 1] Sequence
          (if (not (== _lastkeypressed_3 "None"))
            (bind _keypressed_2 (`self.CheckForInput` _lastkeypressed_3 (`|GetArrayItem` (`self.CurrentRequiredButtons`) (`self.ButtonSequenceIndex`))))
            (if _keypressed_2
              (bind _output_get (set `self.ButtonSequenceIndex` (+ _buttonsequenceindex 1)))
              (if (>= _output_get (`self.ButtonSequenceTotal`))
                (`self.FinishEventHandling`)
                (else
                  (`/Game/Widgets/W_QuickTimeEvent.HandleCorrectSequencePress` (`self.QuickTimeEventWidget`) _buttonsequenceindex)
                  (set `self.LastKeyPressed` "None")))
              (else
                (set `self.LastKeyPressed` "None")
                (if (not (== (`self.ButtonSequenceIndex`) 0))
                  (set `self.ButtonSequenceIndex` 0)
                  (`/Game/Widgets/W_QuickTimeEvent.HandleIncorrectSequencePress` (`self.QuickTimeEventWidget`) (`self.CurrentRequiredButtons`) (`/Game/Blueprints/Player/BP_PlayerCharacter.IsConsolePlayer` (`self.PlayerRef`))))))))
        (:`NewEnumerator2`
          ;[1 1 1] Handle Single Button
          (if (not (== _lastkeypressed "None"))
            (bind _keypressed_3 (`self.CheckForInput` _lastkeypressed (`|GetArrayItem` (`self.CurrentRequiredButtons`) (`self.ButtonSequenceIndex`))))
            (if _keypressed_3
              (`self.FinishEventHandling`))
            (set `self.LastKeyPressed` "None")))))))

(event `SetButtonPress`
  (params (PressedKey :type "Key Structure" :default "None"))
  ;[1 1 1] SetButtonPress
  (set `self.LastKeyPressed` PressedKey))

(event `SetQuickTimeEvent`
  (params (NewQuickTimeEvent :type "/Game/Blueprints/Player/E_EventType Enum" :default "NewEnumerator0") (Interactable :type "Actor Object Reference") (Player :type "/Game/Blueprints/Player/BP_PlayerCharacter Object Reference") (SequenceAmount :type Integer))
  (bind _availablebuttons (`self.AvailableButtons`))
  ;[1 1 1] SetQuickTimeEvent
  (if (not (`self.EventActive`))
    (`self.CreateInteractionWidget` (`Actor.K2_GetActorLocation` Interactable))
    (`/Game/Widgets/W_QuickTimeEvent.SetupEventWidget` (`self.QuickTimeEventWidget`) NewQuickTimeEvent SequenceAmount)
    (set `self.PlayerRef` Player)
    (set `self.EventActive` true)
    (set `self.LastKeyPressed` "None")
    (bind _output_get (set `self.CurrentQuickTimeEvent` NewQuickTimeEvent))
    (switch `/Game/Blueprints/Player/E_EventType` _output_get
      (:`NewEnumerator0`
        (bind _sequenceoutput (`self.GenerateButtonsSequence` _availablebuttons 1))
        ;[1 1 1] Setting ButtonMash
        (if (> (`KismetArrayLibrary.Array_Length` _sequenceoutput) 0)
          (bind _output_get_2 (set `self.CurrentRequiredButtons` _sequenceoutput))
          (`/Game/Widgets/W_QuickTimeEvent.AddButtonPressed` (`self.QuickTimeEventWidget`) (`/Game/Blueprints/Player/BP_PlayerCharacter.IsConsolePlayer` (`self.PlayerRef`)) _output_get_2)
          (set `self.TotalButtonPressCount` 1.0)
          (set `self.ButtonPressCount` 0.0)
          (set `self.FailedEvent` false)
          (else
            (`KismetSystemLibrary.PrintString` "NO Button passed along!" true true (struct :`R` 1.0 :`B` 0.020756 :`A` 1.0)))))
      (:`NewEnumerator1`
        (bind _sequenceoutput_2 (`self.GenerateButtonsSequence` _availablebuttons SequenceAmount))
        ;[1 1 1] Setting Button Sequence
        (if (> (`KismetArrayLibrary.Array_Length` _sequenceoutput_2) 0)
          (bind _output_get_3 (set `self.CurrentRequiredButtons` _sequenceoutput_2))
          (`/Game/Widgets/W_QuickTimeEvent.AddButtonPressed` (`self.QuickTimeEventWidget`) (`/Game/Blueprints/Player/BP_PlayerCharacter.IsConsolePlayer` (`self.PlayerRef`)) _output_get_3)
          (set `self.FailedEvent` false)
          (set `self.ButtonSequenceTotal` (`KismetArrayLibrary.Array_Length` _output_get_3))
          (set `self.ButtonSequenceIndex` 0)
          (else
            (`KismetSystemLibrary.PrintString` "NO Button passed along!" true true (struct :`R` 1.0 :`B` 0.020756 :`A` 1.0)))))
      (:`NewEnumerator2`
        (bind _sequenceoutput_3 (`self.GenerateButtonsSequence` _availablebuttons 1))
        ;[1 1 1] Setting Button Press
        (if (> (`KismetArrayLibrary.Array_Length` _sequenceoutput_3) 0)
          (bind _output_get_4 (set `self.CurrentRequiredButtons` _sequenceoutput_3))
          (`/Game/Widgets/W_QuickTimeEvent.AddButtonPressed` (`self.QuickTimeEventWidget`) (`/Game/Blueprints/Player/BP_PlayerCharacter.IsConsolePlayer` (`self.PlayerRef`)) _output_get_4)
          (set `self.FailedEvent` false)
          (set `self.ButtonSequenceTotal` (`KismetArrayLibrary.Array_Length` _output_get_4))
          (set `self.ButtonSequenceIndex` 0)
          (else
            (`KismetSystemLibrary.PrintString` "NO Button passed along!" true true (struct :`R` 1.0 :`B` 0.020756 :`A` 1.0))))))))

(event `FinishEventHandling`
  ;[1 1 1] FinishEvent
  (`Actor.K2_DestroyActor` (`self.CurrentWidget`))
  (set `self.QuickTimeEventWidget` null)
  (set `self.CurrentWidget` null)
  (`KismetSystemLibrary.PrintString` (`KismetStringLibrary.Concat_StrStr` "Finished event - " (`|GetEnumeratorNameAsString` (`self.CurrentQuickTimeEvent`))))
  (set `self.LastKeyPressed` "None")
  (`/Game/Blueprints/Player/BP_PlayerCharacter.FinishEvent` (`self.PlayerRef`) true)
  (set `self.EventActive` false)
  (set `self.FailedEvent` false))

(fn `ButtonFail`
  (set `self.FailedEvent` true)
  (set `self.EventActive` false)
  (set `self.LastKeyPressed` (struct))
  (`KismetSystemLibrary.PrintString` (`KismetStringLibrary.Concat_StrStr` "Failed the event - " (`|GetEnumeratorNameAsString` (`self.CurrentQuickTimeEvent`)))))

(fn `CheckForInput`
  (params (Key :type "Key Structure (by ref)") (Selection :type "/Game/Blueprints/QuickTimeEvents/QuickTimeEventButtonIndex Enum" :default "NewEnumerator0"))
  (returns (KeyPressed :type Boolean))
  (locals (QuicktimeEv :type "Array of /Game/Blueprints/QuickTimeEvents/QuickTimeEventButtonBindings Structure") (SelectedQuickTime :type "/Game/Blueprints/QuickTimeEvents/QuickTimeEventButtonIndex Enum" :default "NewEnumerator4"))
  (bind _quicktimeev (`local.QuicktimeEv`))
  (bind _quicktimeev_2 (`local.QuicktimeEv`))
  (bind (_output_keybindingindex1 _output_keybindingindex2 _output_keybindingindex3 _output_keybindingindex4) (break `/Game/Blueprints/QuickTimeEvents/QuickTimeEventButtonBindings` (`|GetArrayItem` _quicktimeev_2)))
  (bind _output_keybindingindex1_2 (break `/Game/Blueprints/QuickTimeEvents/QuickTimeEventButtonBindings` (`|GetArrayItem` _quicktimeev)))
  (bind (_output_keybindingindex1_3 _output_keybindingindex2_2) (break `/Game/Blueprints/QuickTimeEvents/QuickTimeEventButtonBindings` (`|GetArrayItem` _quicktimeev)))
  (bind (_output_keybindingindex1_4 _output_keybindingindex2_3 _output_keybindingindex3_2) (break `/Game/Blueprints/QuickTimeEvents/QuickTimeEventButtonBindings` (`|GetArrayItem` _quicktimeev_2)))
  (if (`|EnumEquality` Selection "NewEnumerator4")
    (bind _output_get (set `local.SelectedQuickTime` (`|GetArrayItem` (`self.CurrentRequiredButtons`))))
    (else
      (set `local.SelectedQuickTime` Selection)))
  (switch `/Game/Blueprints/QuickTimeEvents/QuickTimeEventButtonIndex` _output_get
    (:`NewEnumerator0`
      (return (or (== (`|GetArrayItem` _output_keybindingindex1_2) Key) (== (`|GetArrayItem` _output_keybindingindex1_2 1) Key))))
    (:`NewEnumerator1`
      (return (or (== (`|GetArrayItem` _output_keybindingindex2_2) Key) (== (`|GetArrayItem` _output_keybindingindex2_2 1) Key))))
    (:`NewEnumerator2`
      (return (or (== (`|GetArrayItem` _output_keybindingindex3_2) Key) (== (`|GetArrayItem` _output_keybindingindex3_2 1) Key))))
    (:`NewEnumerator3`
      (return (or (== (`|GetArrayItem` _output_keybindingindex4) Key) (== (`|GetArrayItem` _output_keybindingindex4 1) Key))))))

(fn `CreateInteractionWidget`
  (params (SpawningLocation :type "Vector Structure"))
  (bind _returnvalue (`|SpawnActorFromClass` "/Game/Blueprints/QuickTimeEvents/BP_InteractiveWidget.BP_InteractiveWidget_C" (`KismetMathLibrary.MakeTransform` SpawningLocation) "Undefined" "OverrideRootScale" null null))
  (bind _output_get (set `self.CurrentWidget` _returnvalue))
  (set `self.QuickTimeEventWidget` (`/Game/Blueprints/QuickTimeEvents/BP_InteractiveWidget.WidgetRef` _output_get)))

(fn `GenerateButtonsSequence`
  (params (ButtonsToUse :type "Array of /Game/Blueprints/QuickTimeEvents/QuickTimeEventButtonIndex Enum") (SequenceLength :type Integer))
  (returns (sequenceOutput :type "Array of /Game/Blueprints/QuickTimeEvents/QuickTimeEventButtonIndex Enum"))
  (locals (GeneratedButtons :type "Array of /Game/Blueprints/QuickTimeEvents/QuickTimeEventButtonIndex Enum"))
  ;[1 1 1] Generate n amount of buttons based on passed key values
  (for _ (range 1 (+ SequenceLength 1))
    (`KismetArrayLibrary.Array_Add` (`local.GeneratedButtons`) (`|GetArrayItem` ButtonsToUse (`KismetMathLibrary.RandomIntegerInRange` 0 (- (`KismetArrayLibrary.Array_Length` ButtonsToUse) 1)))))
  (return (`local.GeneratedButtons`)))

(fn `SubtractTotalButtonPress`
  (params (LoweringValue :type "Float (double-precision) (by ref)"))
  (bind _buttonpresscount (`self.ButtonPressCount`))
  (if (> _buttonpresscount 0.0)
    (if (>= _buttonpresscount LoweringValue)
      (set `self.ButtonPressCount` (- _buttonpresscount LoweringValue))
      (else
        (set `self.ButtonPressCount` 0.0)))))