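; BP_Barrier is an obstacle actor that rotates a barrier around its pivot when its Activate event fires.
; Activate enables a timer on Tick, which accumulates delta time clamped to one, so the motion lasts about a second.
; The timer linearly blends the pivot's world pitch between two configured angles, zeroing roll and yaw.
; Updates stop once the timer completes, with no reverse or reset logic.
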(event `self.ReceiveTick`
  (params (DeltaSeconds :type "Float (single-precision)"))
  (`parent.ReceiveTick` DeltaSeconds)
  (if (`self.CanUpdateTimer`)
    (`self.UpdateBarrierTimer` DeltaSeconds)
    (`self.MoveBarrier`)
    (if (<= 1.0 (`self.BarrierTimer`))
      (set `self.CanUpdateTimer` false))))

(event `/Game/Blueprints/I_Interaction.Activate`
  (params (Player :type "/Game/Blueprints/Player/BP_PlayerCharacter Object Reference"))
  (set `self.CanUpdateTimer` true))

(fn `MoveBarrier`
  (bind (_x _y) (`KismetMathLibrary.BreakVector2D` (`self.MinMaxRotationBarrier`)))
  (`SceneComponent.K2_SetWorldRotation` (`self.BarrierPivit`) (`KismetMathLibrary.MakeRotator` 0.0 (`KismetMathLibrary.Lerp` _x _y (`self.BarrierTimer`))) false false))

(fn `UpdateBarrierTimer`
  (params (DeltaTime :type "Float (double-precision)"))
  (set `self.BarrierTimer` (`KismetMathLibrary.FClamp` (+ DeltaTime (`self.BarrierTimer`)))))

(fn `UserConstructionScript`
  (`parent.UserConstructionScript`))