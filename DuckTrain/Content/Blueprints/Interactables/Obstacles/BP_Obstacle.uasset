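; Base interactable obstacle that players clear when their inventory holds enough of the required resources.
; Interact checks ResourcesNeeded against the player's inventory, then either starts a button event on the player and hides the requirements widget, or fills that widget once with resource entries.
; Activate destroys destroyable obstacles; otherwise it disables the interaction collider and calls OnActivate, an empty hook for child behaviour.
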(event `/Game/Blueprints/I_Interaction.Activate`
  (params (Player :type "/Game/Blueprints/Player/BP_PlayerCharacter Object Reference"))
  (if (`self.IsDestroyable`)
    (`self.K2_DestroyActor`)
    (else
      (`PrimitiveComponent.SetCollisionEnabled` (`self.InteractionCollider`) "NoCollision")
      (`self.OnActivate`))))

(event `/Game/Blueprints/I_Interaction.Interact`
  (params (Player :type "/Game/Blueprints/Player/BP_PlayerCharacter Object Reference"))
  (bind _value (`self.CanPlayerInteract` Player))
  (if _value
    (bind _asw_resource_requirements (cast `/Game/Widgets/W_ResourceRequirements` (`WidgetComponent.GetUserWidgetObject` (`self.DisplayRequirements`))))
    (set `self.WidgetRef` _asw_resource_requirements)
    (bind _allmet (`self.CheckForRequirementsComplete` Player))
    (if _allmet
      (`/Game/Blueprints/Player/BP_PlayerCharacter.SetupEvent` Player (`self.EventType`) (`self.RequiredButtons`))
      (`SceneComponent.SetVisibility` (`self.DisplayRequirements`) false false)
      (elif (`self.WidgetSetup`)
        (`self.SetInteractRequirements` Player)
        (set `self.WidgetSetup` false)))))

(fn `CheckForRequirementsComplete`
  (params (PlayerRef :type "/Game/Blueprints/Player/BP_PlayerCharacter Object Reference"))
  (returns (AllMet :type Boolean))
  (locals (AllRequirementsMet :type Boolean :default true) (RequiredNumbers :type "Array of Integer"))
  (bind _resourcesneeded (`self.ResourcesNeeded`))
  (bind _values (`BlueprintMapLibrary.Map_Values` _resourcesneeded))
  (set `local.RequiredNumbers` _values)
  (bind _keys (`BlueprintMapLibrary.Map_Keys` _resourcesneeded))
  (for (_array_element _array_index) _keys
    (bind _value (`/Game/Blueprints/Player/Cmp_Inventory.GetValueInInventory` (`/Game/Blueprints/Player/BP_PlayerCharacter.Cmp_Inventory` PlayerRef) _array_element))
    (if (not (>= _value (`|GetArrayItem` (`local.RequiredNumbers`) _array_index)))
      (set `local.AllRequirementsMet` false)))
  (return (`local.AllRequirementsMet`)))

(fn `OnActivate`)

(fn `SetInteractRequirements`
  (params (PlayerRef :type "/Game/Blueprints/Player/BP_PlayerCharacter Object Reference"))
  (locals (RequiredNumbers :type "Array of Integer"))
  (bind _resourcesneeded (`self.ResourcesNeeded`))
  (bind _values (`BlueprintMapLibrary.Map_Values` _resourcesneeded))
  (set `local.RequiredNumbers` _values)
  (bind _keys (`BlueprintMapLibrary.Map_Keys` _resourcesneeded))
  (for (_array_element _array_index) _keys
    (bind _returnvalue (`|CreateWidget` "/Game/Widgets/W_Resource.W_Resource_C"))
    (`PanelWidget.AddChild` (`/Game/Widgets/W_ResourceRequirements.HorenzotalBar` (`self.WidgetRef`)) _returnvalue)
    (`/Game/Widgets/W_Resource.SetAmount` _returnvalue (`|GetArrayItem` (`local.RequiredNumbers`) _array_index))
    (`/Game/Widgets/W_Resource.SetResourceName` _returnvalue _array_element)))

(fn `UserConstructionScript`)