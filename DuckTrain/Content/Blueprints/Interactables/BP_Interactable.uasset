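; BP_Interactable is an interactable actor that starts an event on the player who interacts with it, restricted to Player 1, Player 2 or both.
; Interact asks CanPlayerInteract, which checks the PlayerInteractable setting and compares the caller to the player character at index 0 or 1.
; When allowed, it passes its EventType and RequiredButtons count to the player's SetupEvent, leaving the event itself to the player.
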(event `/Game/Blueprints/I_Interaction.Interact`
  (params (Player :type "/Game/Blueprints/Player/BP_PlayerCharacter Object Reference"))
  (bind _value (`self.CanPlayerInteract` Player))
  (if _value
    (`/Game/Blueprints/Player/BP_PlayerCharacter.SetupEvent` Player (`self.EventType`) (`self.RequiredButtons`))))

(fn `CanPlayerInteract`
  (params (Player :type "/Game/Blueprints/Player/BP_PlayerCharacter Object Reference"))
  (returns (Value :type Boolean))
  (locals (NewLocalVar_0 :type "/Game/Blueprints/Player/BP_PlayerCharacter Object Reference"))
  (switch `/Game/Blueprints/Interactables/E_PlayerInteractable` (`self.PlayerInteractable`)
    (:`NewEnumerator0`
      (bind _asbp_player_character (cast `/Game/Blueprints/Player/BP_PlayerCharacter` (`GameplayStatics.GetPlayerCharacter` 0)))
      (if (== _asbp_player_character (`local.Player`))
        (return true)))
    (:`NewEnumerator1`
      (bind _asbp_player_character_2 (cast `/Game/Blueprints/Player/BP_PlayerCharacter` (`GameplayStatics.GetPlayerCharacter` 1)))
      (if (== _asbp_player_character_2 (`local.Player`))
        (return true)))
    (:`NewEnumerator2`
      (return true))))

(fn `UserConstructionScript`)