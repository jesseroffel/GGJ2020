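; BP_Resource is an interactable resource pickup that a player can carry.
; On Activate, it flags the player as carrying an item, passes its ResourceType to the player's inventory component as the current resource, then destroys itself.
; It has no active BeginPlay, overlap or Tick logic, so all behavior runs through that single event.
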(event `/Game/Blueprints/I_Interaction.Activate`
  (params (Player :type "/Game/Blueprints/Player/BP_PlayerCharacter Object Reference"))
  (set `/Game/Blueprints/Player/BP_PlayerCharacter.IsCarryingItem` true Player)
  (`/Game/Blueprints/Player/Cmp_Inventory.SetCurrentResourceType` (`/Game/Blueprints/Player/BP_PlayerCharacter.Cmp_Inventory` Player) (`self.ResourceType`))
  (`self.K2_DestroyActor`))

(fn `UserConstructionScript`
  (`parent.UserConstructionScript`))