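; Train actor that drives itself along its forward vector, slowing to a halt for obstacles and pulling away when the path clears.
; Each tick it updates an acceleration alpha, runs a stop check and moves, scaling speed through an acceleration curve.
; The stop check uses an ObstacleCheck macro, a forward line trace with Hit and No Hit exits.
; Interacting adds one unit of the player's current resource type to their inventory.
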(event `self.ReceiveTick`
  (params (DeltaSeconds :type "Float (single-precision)"))
  (`|ExecutionSequence`
    (:`then_0`
      (if (`self.IsAccelerating`)
        (`self.Accelerate` DeltaSeconds)
        (elif (`self.IsDecelerating`)
          (`self.Decelerate` DeltaSeconds))))
    (:`then_1`
      (`self.StopCheck`))
    (:`then_2`
      (`self.Move` DeltaSeconds))))

(event `/Game/Blueprints/I_Interaction.Interact`
  (params (Player :type "/Game/Blueprints/Player/BP_PlayerCharacter Object Reference"))
  (bind _cmp_inventory (`/Game/Blueprints/Player/BP_PlayerCharacter.Cmp_Inventory` Player))
  (bind _resourcetype (`/Game/Blueprints/Player/Cmp_Inventory.GetCurrentResourceType` _cmp_inventory))
  (`/Game/Blueprints/Player/Cmp_Inventory.AddValueToInventory` _cmp_inventory _resourcetype 1))

(fn `Accelerate`
  (params (DeltaTime :type "Float (double-precision)"))
  (bind _returnvalue (+ (* DeltaTime (`self.AccelerationSpeed`)) (`self.Acceleration`)))
  (if (>= _returnvalue 1.0)
    (set `self.Acceleration` 1.0)
    (set `self.IsAccelerating` false)
    (else
      (set `self.Acceleration` _returnvalue))))

(fn `Decelerate`
  (params (DeltaTime :type "Float (double-precision)"))
  (bind _returnvalue (- (`self.Acceleration`) (* DeltaTime (`self.DecelerationSpeed`))))
  (if (<= _returnvalue 0.0)
    (set `self.Acceleration` 0.0)
    (set `self.IsDecelerating` false)
    (set `self.CanMove` false)
    (else
      (set `self.Acceleration` _returnvalue))))

(fn `Move`
  (params (DeltaTime :type "Float (double-precision)"))
  (if (`self.CanMove`)
    (`self.K2_SetActorLocation` (+ (`self.K2_GetActorLocation`) (* (`self.GetActorForwardVector`) (* (`local.DeltaTime`) (`self.MovementSpeed`) (`CurveFloat.GetFloatValue` (`self.AccelerationCurve`) (`self.Acceleration`))))))))

(fn `StopCheck`
  (if (and (`self.CanMove`) (not (`self.IsDecelerating`)))
    (`self.ObstacleCheck`
      (:`Hit`
        (set `self.IsDecelerating` true)
        (set `self.IsAccelerating` false)))
    (else
      (`self.ObstacleCheck`
        (:`No Hit`
          (set `self.CanMove` true)
          (set `self.IsAccelerating` true))))))

(fn `UserConstructionScript`)