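; Game mode for a local two-player train game with resources, scores and an end screen.
; StartGamemode spawns and possesses both characters, creates the HUD and finds each player's train.
; In L_Game, Tick refreshes resource counts and, at shared checkpoints, updates scores, releases both trains when ready or shows final results.
; Helper functions build a pool of random button events with resource costs and randomly assign them to each player's interactables.
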(event `StartGamemode`
  (bind _returnvalue (`GameplayStatics.GetPlayerController` 0))
  (`WidgetBlueprintLibrary.SetInputMode_GameAndUIEx` _returnvalue null)
  (bind _returnvalue_2 (`|SpawnActorFromClass` "/Game/Blueprints/Player/BP_PlayerCharacter.BP_PlayerCharacter_C" (`KismetMathLibrary.MakeTransform` (`self.SpawnLocationPlayer1`)) "Undefined" "OverrideRootScale" null null))
  (`Controller.Possess` _returnvalue _returnvalue_2)
  (`GameplayStatics.CreatePlayer` -1)
  (bind _returnvalue_3 (`|SpawnActorFromClass` "/Game/Blueprints/Player/BP_PlayerCharacter.BP_PlayerCharacter_C" (`KismetMathLibrary.MakeTransform` (`self.SpawnLocationPlayer2`)) "Undefined" "OverrideRootScale" null null))
  (`Controller.Possess` (`GameplayStatics.GetPlayerController` 1) _returnvalue_3)
  (bind _asbp_player_character (cast `/Game/Blueprints/Player/BP_PlayerCharacter` (`GameplayStatics.GetPlayerPawn` 0))
    (:`then`
      (bind _output_get (set `self.Player1` _asbp_player_character))
      (set `/Game/Blueprints/Player/BP_PlayerCharacter.PlayerID` 0 _output_get))
    (:`CastFailed`
      (`KismetSystemLibrary.PrintString` "Player1 Not Found" true true (struct :`R` 1.0 :`A` 1.0))))
  (bind _asbp_player_character_2 (cast `/Game/Blueprints/Player/BP_PlayerCharacter` (`GameplayStatics.GetPlayerPawn` 1))
    (:`then`
      (bind _output_get_2 (set `self.Player2` _asbp_player_character_2))
      (set `/Game/Blueprints/Player/BP_PlayerCharacter.PlayerID` 1 _output_get_2))
    (:`CastFailed`
      (`KismetSystemLibrary.PrintString` "Player2 Not Found" true true (struct :`R` 1.0 :`A` 1.0))))
  (bind _returnvalue_4 (`|CreateWidget` "/Game/Widgets/W_HUD.W_HUD_C"))
  (bind _output_get_3 (set `self.HUDReference` _returnvalue_4))
  (`UserWidget.AddToViewport` _output_get_3 0)
  (bind _outactors (`GameplayStatics.GetAllActorsOfClass` "/Game/Blueprints/Train/BP_Train.BP_Train_C"))
  (for _array_element _outactors
    (bind _playerid (`/Game/Blueprints/Train/BP_Train.PlayerID` _array_element))
    (if (== 0 _playerid)
      (set `self.TrainPlayer1` _array_element)
      (elif (== _playerid 1)
        (set `self.TrainPlayer2` _array_element)))))

(event `self.ReceiveTick`
  (params (DeltaSeconds :type "Float (single-precision)"))
  (bind _returnvalue (`GameplayStatics.GetCurrentLevelName` true))
  (if (`KismetStringLibrary.EqualEqual_StrStr` _returnvalue "L_Game")
    (`self.UpdateHUD`)
    (`self.UpdateTrainCheckpoint`)))

(fn `CreateRandomEvents`
  (params (Amount :type Integer))
  (bind (_x _y) (`KismetMathLibrary.BreakVector2D` (`self.ButtonSequenceMinMax`)))
  (bind (_x_2 _y_2) (`KismetMathLibrary.BreakVector2D` (`self.ButtonMeshMinMax`)))
  (bind _returnvalue (cast `/Game/Blueprints/Player/E_EventType` (`KismetMathLibrary.Conv_IntToByte` (`KismetMathLibrary.RandomIntegerInRange` 0 (enumcount `/Game/Blueprints/Player/E_EventType`)))))
  (for _ (range (+ Amount 1))
    (switch `/Game/Blueprints/Player/E_EventType` _returnvalue
      (:`NewEnumerator0`
        (bind _resources (`self.GetRandomResources`))
        (`KismetArrayLibrary.Array_Add` (`self.PlayersInteractables`) (make `/Game/Blueprints/Interactables/S_InteractableData` _returnvalue (`KismetMathLibrary.RandomIntegerInRange` (`KismetMathLibrary.FTrunc` _x_2) (`KismetMathLibrary.FTrunc` _y_2)) _resources)))
      (:`NewEnumerator1`
        (bind _resources_2 (`self.GetRandomResources`))
        (`KismetArrayLibrary.Array_Add` (`self.PlayersInteractables`) (make `/Game/Blueprints/Interactables/S_InteractableData` _returnvalue (`KismetMathLibrary.RandomIntegerInRange` (`KismetMathLibrary.FTrunc` _x) (`KismetMathLibrary.FTrunc` _y)) _resources_2)))
      (:`NewEnumerator2`
        (bind _resources_3 (`self.GetRandomResources`))
        (`KismetArrayLibrary.Array_Add` (`self.PlayersInteractables`) (make `/Game/Blueprints/Interactables/S_InteractableData` _returnvalue 1 _resources_3))))))

(fn `GetRandomResources`
  (returns (Resources :type "Map of /Game/Blueprints/Player/E_ResourceType Enum to Integer"))
  (locals (ResourceTypes :type "Array of /Game/Blueprints/Player/E_ResourceType Enum") (ResourceAmount :type "Map of /Game/Blueprints/Player/E_ResourceType Enum to Object Object Reference") (Amount :type Integer :default 4) (Resource :type "/Game/Blueprints/Player/E_ResourceType Enum") (RandomInt :type Integer))
  (bind _resourceamount (`local.ResourceAmount`))
  (bind _resourcetypes (`local.ResourceTypes`))
  (bind _resourcetypes_2 (`local.ResourceTypes`))
  (set `local.ResourceTypes` (`|MakeArray` "NewEnumerator1" "NewEnumerator2" "NewEnumerator3" :!type "/Game/Blueprints/Player/E_ResourceType Enum"))
  (set `local.Amount` 3)
  (for _ (range (+ (`KismetArrayLibrary.Array_LastIndex` (`local.ResourceTypes`)) 1))
    (set `local.Resource` (`|GetArrayItem` _resourcetypes (`KismetMathLibrary.RandomIntegerInRange` 0 (`KismetArrayLibrary.Array_LastIndex` _resourcetypes))))
    (set `local.RandomInt` (`KismetMathLibrary.RandomIntegerInRange` 0 (`local.Amount`)))
    (`BlueprintMapLibrary.Map_Add` (`local.ResourceAmount`) (`local.Resource`) (`local.RandomInt`))
    (`KismetArrayLibrary.Array_RemoveItem` (`local.ResourceTypes`) (`local.Resource`))
    (set `local.Amount` (- (`local.Amount`) (`local.RandomInt`))))
  (`BlueprintMapLibrary.Map_Add` (`local.ResourceAmount`) (`|GetArrayItem` _resourcetypes_2 (`KismetMathLibrary.RandomIntegerInRange` 0 (`KismetArrayLibrary.Array_LastIndex` _resourcetypes_2))) (`local.Amount`))
  (bind _keys (`BlueprintMapLibrary.Map_Keys` (`local.ResourceAmount`)))
  (for _array_element _keys
    (if (== (`BlueprintMapLibrary.Map_Find` (`local.ResourceAmount`) _array_element) 0)
      (`BlueprintMapLibrary.Map_Remove` _resourceamount _array_element)))
  (return _resourceamount))

(fn `GiveRandomEventsToInteractables`
  (params (Player1Interactables :type "Array of /Game/Blueprints/Interactables/BP_Interactable Object Reference") (Player2Interactables :type "Array of /Game/Blueprints/Interactables/BP_Interactable Object Reference"))
  (`self.CreateRandomEvents` (+ (`KismetArrayLibrary.Array_Length` Player1Interactables) 1))
  (`self.SetupInteractables` (`self.PlayersInteractables`) Player1Interactables)
  (`self.SetupInteractables` (`self.PlayersInteractables`) Player2Interactables "NewEnumerator1"))

(fn `SetHUDInfoPlayer`
  (params (`HUD element` :type "/Game/Widgets/W_PlayerResources Object Reference") (Player :type "/Game/Blueprints/Player/BP_PlayerCharacter Object Reference"))
  (`self.SetResourceAmount` (`/Game/Widgets/W_PlayerResources.W_Resource1` `HUD element`) (`local.Player`) "NewEnumerator1")
  (`self.SetResourceAmount` (`/Game/Widgets/W_PlayerResources.W_Resource2` `HUD element`) (`local.Player`) "NewEnumerator2")
  (`self.SetResourceAmount` (`/Game/Widgets/W_PlayerResources.W_Resource3` `HUD element`) (`local.Player`) "NewEnumerator3"))

(fn `SetPlayerToSpawnLocation`
  (for (_array_element _array_index) (`|MakeArray` (`GameplayStatics.GetPlayerCharacter` 0) (`GameplayStatics.GetPlayerCharacter` 1))
    (`SceneComponent.K2_SetWorldTransform` (`Actor.RootComponent` _array_element) (`KismetMathLibrary.MakeTransform` (`|GetArrayItem` (`|MakeArray` (`self.SpawnLocationPlayer1`) (`self.SpawnLocationPlayer2`)) _array_index)) false true)))

(fn `SetResourceAmount`
  (params (Widget :type "/Game/Widgets/W_Resource Object Reference") (Player :type "/Game/Blueprints/Player/BP_PlayerCharacter Object Reference") (ResourceType :type "/Game/Blueprints/Player/E_ResourceType Enum" :default "NewEnumerator0"))
  (bind _value (`/Game/Blueprints/Player/Cmp_Inventory.GetValueInInventory` (`/Game/Blueprints/Player/BP_PlayerCharacter.Cmp_Inventory` Player) ResourceType))
  (`/Game/Widgets/W_Resource.SetAmount` Widget _value))

(fn `SetupInteractables`
  (params (PlayerInteractables :type "Array of /Game/Blueprints/Interactables/S_InteractableData Structure") (InputPin :type "Array of /Game/Blueprints/Interactables/BP_Interactable Object Reference") (PlayerInteractable :type "/Game/Blueprints/Interactables/E_PlayerInteractable Enum" :default "NewEnumerator0"))
  (locals (PlayerinteractablesInstance :type "Array of /Game/Blueprints/Interactables/S_InteractableData Structure"))
  (bind _output (`|GetArrayItem` (`local.PlayerinteractablesInstance`) (`KismetMathLibrary.RandomIntegerInRange` 0 (`KismetArrayLibrary.Array_LastIndex` (`local.PlayerinteractablesInstance`)))))
  (bind (_eventtype _buttonamount _resourceamount) (break `/Game/Blueprints/Interactables/S_InteractableData` _output))
  (set `local.PlayerinteractablesInstance` PlayerInteractables)
  (for _array_element InputPin
    (set `/Game/Blueprints/Interactables/BP_Interactable.PlayerInteractable` PlayerInteractable _array_element)
    (set `/Game/Blueprints/Interactables/BP_Interactable.EventType` _eventtype _array_element)
    (set `/Game/Blueprints/Interactables/BP_Interactable.RequiredButtons` _buttonamount _array_element)
    (set `/Game/Blueprints/Interactables/BP_Interactable.ResourcesNeeded` _resourceamount _array_element)
    (`KismetArrayLibrary.Array_RemoveItem` (`local.PlayerinteractablesInstance`) _output)))

(fn `UpdateHUD`
  (bind _player2 (`self.Player2`))
  (bind _player1 (`self.Player1`))
  (bind _w_player1resources (`/Game/Widgets/W_HUD.W_Player1Resources` (`self.HUDReference`)))
  (bind _w_player2resources (`/Game/Widgets/W_HUD.W_Player2Resources` (`self.HUDReference`)))
  (`|ExecutionSequence`
    (:`then_0`
      (if (and (`KismetSystemLibrary.IsValid` _w_player1resources) (`KismetSystemLibrary.IsValid` _player1))
        (`self.SetHUDInfoPlayer` _w_player1resources _player1)))
    (:`then_1`
      (if (and (`KismetSystemLibrary.IsValid` _w_player2resources) (`KismetSystemLibrary.IsValid` _player2))
        (`self.SetHUDInfoPlayer` _w_player2resources _player2)))))

(fn `UpdateScores`
  (`/Game/Widgets/W_HUD.UpdateScores` (`self.HUDReference`) (`/Game/Blueprints/Player/BP_PlayerCharacter.Score` (`self.Player1`)) (`/Game/Blueprints/Player/BP_PlayerCharacter.Score` (`self.Player2`))))

(fn `UpdateTrainCheckpoint`
  (bind _trainplayer1 (`self.TrainPlayer1`))
  (bind _trainplayer2 (`self.TrainPlayer2`))
  (if (and (`/Game/Blueprints/Train/BP_Train.IsAtCheckpoint` (`self.TrainPlayer1`)) (`/Game/Blueprints/Train/BP_Train.IsAtCheckpoint` (`self.TrainPlayer2`)))
    (`self.UpdateScores`)
    (if (and (`/Game/Blueprints/Train/BP_Train.IsAtFinalCheckpoint` (`self.TrainPlayer1`)) (`/Game/Blueprints/Train/BP_Train.IsAtFinalCheckpoint` (`self.TrainPlayer2`)))
      (if (not (`self.IsDisplayingEndScreen`))
        (bind _returnvalue (`|CreateWidget` "/Game/Widgets/W_EndScreen.W_EndScreen_C"))
        (`UserWidget.AddToViewport` _returnvalue 0)
        (`/Game/Widgets/W_EndScreen.SetScore` _returnvalue (`/Game/Blueprints/Player/BP_PlayerCharacter.Score` (`self.Player1`)) (`/Game/Blueprints/Player/BP_PlayerCharacter.Score` (`self.Player2`)))
        (`WidgetBlueprintLibrary.SetInputMode_UIOnlyEx` (`GameplayStatics.GetPlayerController` 0) _returnvalue)
        (set `self.IsDisplayingEndScreen` true))
      (elif (and (`/Game/Blueprints/Train/BP_Train.IsReadyToLeave` (`self.TrainPlayer1`)) (`/Game/Blueprints/Train/BP_Train.IsReadyToLeave` (`self.TrainPlayer2`)))
        (`|ExecutionSequence`
          (:`then_0`
            (set `/Game/Blueprints/Train/BP_Train.CanMove` true _trainplayer1)
            (set `/Game/Blueprints/Train/BP_Train.IsAccelerating` true _trainplayer1)
            (set `/Game/Blueprints/Train/BP_Train.IsAtCheckpoint` false _trainplayer1))
          (:`then_1`
            (set `/Game/Blueprints/Train/BP_Train.CanMove` true _trainplayer2)
            (set `/Game/Blueprints/Train/BP_Train.IsAccelerating` true _trainplayer2)
            (set `/Game/Blueprints/Train/BP_Train.IsAtCheckpoint` false _trainplayer2)))))))

(fn `UserConstructionScript`)