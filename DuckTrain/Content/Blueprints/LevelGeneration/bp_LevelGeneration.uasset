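; Level generator for a train game that lays out a tiled map with parallel tracks, one train per track.
; The construction script instances grass and gravel tiles and picks tree spots in the edge lanes using 1D Perlin noise.
; BeginPlay spawns trains, trees, evenly spaced checkpoints with obstacles between them, and per-player obstacle lists.
; Track instances are laid last, using recorded obstacle positions to leave gaps.
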(event `self.ReceiveBeginPlay`
  (bind _inteval (`self.inteval`))
  (bind _tilewidth (`self.TileWidth`))
  ;[1 0.05157 0] Spawn train, Choo choo
  (`|ExecutionSequence`
    (:`then_0`
      (for (_array_element _array_index) (`self.TracksVerticals`)
        (`self.SpawnTrain` (`KismetMathLibrary.MakeVector` 0.0 (* _array_element (`self.TileHeight`)) 0.1) _array_index)))
    (:`then_1`
      (`self.SpawnObjects`)
      (`self.SpawnTrees`))
    (:`then_2`
      (for _array_element_2 (`self.TracksVerticals`)
        (set `self.inteval` (- (`KismetArrayLibrary.Array_Length` (`self.NewVar_0`)) 1))
        (for _index (range (`self.TileCountY`))
          (if (== _index (`|GetArrayItem` (`self.NewVar_0`) (`self.inteval`)))
            (`/Engine/EditorBlueprintResources/StandardMacros.DecrementInt` _inteval
              (:`  `
                (if (< _inteval 0)
                  (set `self.inteval` 0))))
            (else
              (`InstancedStaticMeshComponent.AddInstance` (`self.Track`) (`KismetMathLibrary.MakeTransform` (`KismetMathLibrary.MakeVector` (`KismetMathLibrary.Conv_IntToDouble` (* _index (`KismetMathLibrary.FTrunc` _tilewidth))) (`KismetMathLibrary.Conv_IntToDouble` (* _array_element_2 (`KismetMathLibrary.FTrunc` _tilewidth)))) (struct :`Yaw` 90.0))))))))))

(fn `SpawnObjects`
  (locals (NextCheckPointStep :type Integer) (NextCheckPoint :type Integer) (NextObstacleStep :type Integer) (NextObstacle :type Integer))
  (bind _output_get (set `local.NextCheckPointStep` (/ (`self.TileCountY`) (`self.CheckPointCount`))))
  (set `local.NextObstacleStep` (/ _output_get (+ (`self.ObstacleCount`) 1)))
  (for _index (range 1 (+ (`self.CheckPointCount`) 1))
    (`|ExecutionSequence`
      (:`then_0`
        (bind _returnvalue (* _index (`local.NextCheckPointStep`)))
        (bind _output_get_2 (set `local.NextCheckPoint` _returnvalue))
        (for _index_2 (range 1 (+ (`self.ObstacleCount`) 1))
          (bind _returnvalue_2 (- _output_get_2 (* _index_2 (`local.NextObstacleStep`))))
          (`KismetArrayLibrary.Array_Add` (`self.NewVar_0`) _returnvalue_2)
          (for (_array_element _array_index) (`self.TracksVerticals`)
            (bind _returnvalue_3 (`|SpawnActorFromClass` "/Game/Blueprints/Interactables/Obstacles/BP_Obstacle.BP_Obstacle_C" (`KismetMathLibrary.MakeTransform` (`KismetMathLibrary.MakeVector` (* _returnvalue_2 (`self.TileWidth`)) (* _array_element (`self.TileWidth`)) 50.0)) "Undefined" "OverrideRootScale" null null))
            (`KismetArrayLibrary.Array_Add` (select `int` _array_index :`0` (`self.Player1_Obstacle`) :`1` (`self.Player2_Obstacle`)) _returnvalue_3))))
      (:`then_1`
        (for _array_element_2 (`self.TracksVerticals`)
          ;[1 1 1] Add checkpoint
          (bind _returnvalue_4 (`|SpawnActorFromClass` "/Game/Blueprints/Train/BP_Checkpoint.BP_Checkpoint_C" (`KismetMathLibrary.MakeTransform` (`KismetMathLibrary.MakeVector` (* _returnvalue (`self.TileWidth`)) (* _array_element_2 (`self.TileWidth`)))) "Undefined" "OverrideRootScale" null null))
          (if (== _index (`self.CheckPointCount`))
            (set `/Game/Blueprints/Train/BP_Checkpoint.IsFinal` true _returnvalue_4)))))))

(fn `SpawnTrain`
  (params (Position :type "Vector Structure") (PlayerID :type Integer))
  (`|SpawnActorFromClass` "/Game/Blueprints/Train/BP_Train.BP_Train_C" (`KismetMathLibrary.MakeTransform` Position) "Undefined" "OverrideRootScale" null PlayerID null))

(fn `SpawnTrees`
  (for _array_element (`self.Trees`)
    (bind (_x _y) (`KismetMathLibrary.BreakVector2D` _array_element))
    (`|SpawnActorFromClass` "/Game/Blueprints/LevelGeneration/bp_tree0.bp_tree0_C" (`KismetMathLibrary.MakeTransform` (`KismetMathLibrary.MakeVector` (* _y (`self.TileHeight`)) (* _x (`self.TileWidth`))) (`KismetMathLibrary.MakeRotator` 0.0 0.0 (`KismetMathLibrary.RandomFloatInRange` 0.0 360.0))) "Undefined" "OverrideRootScale" null null)))

(fn `UserConstructionScript`
  (locals (NextCheckPointStep :type Integer) (NextCheckPoint :type Integer) (NextObstacleStep :type Integer) (NextObstacle :type Integer) (TrackIDX :type Integer) (Tacks :type Boolean))
  (bind _treespawnlanes (`self.TreeSpawnLanes`))
  (`|ExecutionSequence`
    (:`then_0`
      (for _index (range (`self.TileCountX`))
        (for _index_2 (range (`self.TileCountY`))
          (if (and (or (> _index (- (`self.TileCountX`) _treespawnlanes)) (< _index _treespawnlanes)) (> (* (`self.TreeProbibility`) (* (+ (`KismetMathLibrary.PerlinNoise1D` (* (`KismetMathLibrary.Conv_IntToDouble` (+ _index_2 (* _index (`self.TileCountX`)))) 1.43523)) 1.0) 0.5)) 0.9))
            (`KismetArrayLibrary.Array_Add` (`self.Trees`) (`KismetMathLibrary.MakeVector2D` (`KismetMathLibrary.Conv_IntToDouble` _index) (`KismetMathLibrary.Conv_IntToDouble` _index_2)))))))
    (:`then_1`
      (for _index_3 (range (`self.TileCountY`))
        (for _index_4 (range (`self.TileCountX`))
          (set `local.Tacks` false)
          (for _array_element (`self.TracksVerticals`)
            (if (== _index_4 _array_element)
              (set `local.Tacks` true)))
          (if (`local.Tacks`)
            (bind _returnvalue (`KismetMathLibrary.MakeTransform` (`KismetMathLibrary.MakeVector` (* _index_3 (`self.TileHeight`)) (* _index_4 (`self.TileWidth`))) (struct :`Yaw` 90.0)))
            (`InstancedStaticMeshComponent.AddInstance` (`self.Gravel`) _returnvalue)
            (else
              (`InstancedStaticMeshComponent.AddInstance` (`self.Grass`) _returnvalue))))))))